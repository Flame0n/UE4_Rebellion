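; GameplayPC is a player controller that drives camera movement through its controlled pawn and handles the match-end display.
; Forward and right axis inputs offset the pawn along its own vectors without sweep, while turn input adds yaw.
; Movement and turn steps scale by speed variables but not by delta time.
; When the match ends, it passes the win result to GameHUD to show the end-match widget.
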(event EventEventMatchWasEnded
  (params (IsWin :type Boolean))
  ;[1 1 1] Show widget on match end
  (Default|ShowEndMatchWidget (.AsGame%20HUD (Utilities|Casting|CastToGameHUD (HUD|GetHUD))) IsWin))

(event Input|AxisEvents|InputAxisTurnRate
  (params (AxisValue :type Float%20%28single-precision%29))
  (bind _returnvalue (Pawn|GetControlledPawn))
  ;[1 1 1] Camera Movement
  (Utilities|IsValid _returnvalue
    (:Is%20Valid
      (Class|Actor|AddActorWorldRotation _returnvalue (Math|Rotator|MakeRotator 0.0 0.0 (* AxisValue (Variables|Default|GetTurnSpeed)))))))

(event Input|AxisEvents|InputAxisMoveForward
  (params (AxisValue :type Float%20%28single-precision%29))
  (bind _returnvalue (Pawn|GetControlledPawn))
  ;[1 1 1] Camera Movement
  (Utilities|IsValid _returnvalue
    (:Is%20Valid
      (Transformation|AddActorWorldOffset _returnvalue (* (Transformation|GetActorForwardVector (Pawn|GetControlledPawn)) (* AxisValue (Variables|Default|GetMoveSpeed)))))))

(event Input|AxisEvents|InputAxisMoveRight
  (params (AxisValue :type Float%20%28single-precision%29))
  (bind _returnvalue (Pawn|GetControlledPawn))
  ;[1 1 1] Camera Movement
  (Utilities|IsValid _returnvalue
    (:Is%20Valid
      (Transformation|AddActorWorldOffset _returnvalue (* (Transformation|GetActorRightVector (Pawn|GetControlledPawn)) (* AxisValue (Variables|Default|GetMoveSpeed)))))))

(fn ConstructionScript)