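; Base building actor with an info widget that appears only while the first local player is partway through invading it.
; On BeginPlay it passes itself to the BuildingInfoWidget as owner and starts a looping timer.
; The timer polls the InvadableComponent for that player's invade points, showing the widget only when they are strictly between zero and full.
; A note marks this visibility logic to move into the widget.
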(event Custom|Set%20Visibility
  (bind _returnvalue (Actor|GetComponentbyClass "/Script/Rebellion.InvadableComponent"))
  (bind _returnvalue_2 (Game|GetPlayerController 0))
  (bind _playerstate (Variables|/Script/Engine.Controller|GetPlayerState _returnvalue_2))
  (bind _asgameplay_player_state (Utilities|Casting|CastToGameplayPlayerState _playerstate))
  (bind _returnvalue_3 (Class|InvadableComponent|GetInvadePointsbyPlayer _returnvalue _asgameplay_player_state))
  ;[1 1 1] Move this logic to widget
  (Rendering|SetVisibility (Variables|Default|GetInfo%20Widget) (and (> _returnvalue_3 0.0) (< _returnvalue_3 1e+02)) false))

(event EventBeginPlay
  (bind _asbuilding_info_widget (Utilities|Casting|CastToBuildingInfoWidget (UserInterface|GetUserWidgetObject (Variables|Default|GetInfo%20Widget))))
  (Variables|/Game/Interface/Gameplay/BuildingInfoWidget.BuildingInfoWidget_C|SetOwnerActor _asbuilding_info_widget self)
  (Utilities|Time|SetTimerbyEvent (delegate Custom|Set%20Visibility) 0.2 true)
  (CallFunction|SetVisibility))

(fn ConstructionScript)