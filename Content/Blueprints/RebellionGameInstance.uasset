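; Game instance for Rebellion that manages online session setup and teardown and reports network and travel errors.
; On Init, a dedicated server creates a 10-connection LAN session, and a caller event destroys the session on request.
; Network failures are converted to readable text and printed through DisplayErrorMessage.
; Travel failures print only a fixed "Travel" message, leaving the TravelErrorToString helper unused.
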(event Custom|DestroySessionCaller
  (params (PlayerController :type Player%20Controller%20Object%20Reference))
  ;[1 1 1] Destroy session
  (|DestroySession PlayerController))

(event EventHandleNetworkError
  (params (FailureType :type ENetworkFailure%20Enum :default "NetDriverAlreadyExists") (bIsServer :type Boolean))
  ;[1 1 1] Display message on network error
  (if bIsServer
    _
    (else
      _))
  (Utilities|DisplayErrorMessage (CallFunction|NetErrortoString FailureType)))

(event EventHandleTravelError
  (params (FailureType :type ETravelFailure%20Enum :default "NoLevel"))
  ;[1 1 1] Handle Travel error
  (Utilities|DisplayErrorMessage "Travel"))

(event EventInit
  ;[1 1 1] Launch dedicated server
  (if (Networking|IsDedicatedServer)
    (|Session (Game|GetPlayerController 0) 10 true
      (:OnSuccess
        (Development|PrintString "Session was created"))
      (:OnFailure
        (Development|PrintString "Session creation failed")))))

(fn NetErrortoString
  (params (FailureType :type ENetworkFailure%20Enum :default "NetDriverAlreadyExists"))
  (switch Utilities|FlowControl|Switch|SwitchonENetworkFailure FailureType
    (:NetDriverAlreadyExists
      (LocalVariables|SetResult "Driver already exists"))
    (:NetDriverCreateFailure
      (LocalVariables|SetResult "Driver create failure"))
    (:NetDriverListenFailure
      (LocalVariables|SetResult "Listen Failure"))
    (:ConnectionLost
      (LocalVariables|SetResult "Connection lost"))
    (:ConnectionTimeout
      (LocalVariables|SetResult "Connection timeout"))
    (:FailureReceived
      (LocalVariables|SetResult "Failure recieved"))
    (:OutdatedClient
      (LocalVariables|SetResult "Outdated client"))
    (:OutdatedServer
      (LocalVariables|SetResult "Outdated server"))
    (:PendingConnectionFailure
      (LocalVariables|SetResult "Pending connection fail"))
    (:NetGuidMismatch
      (LocalVariables|SetResult "Net guid mismatch"))
    (:NetChecksumMismatch
      (LocalVariables|SetResult "Net checksum mistmatch")))
  (return (LocalVariables|GetResult)))

(fn TravelErrortoString
  (params (FailureType :type ETravelFailure%20Enum :default "NoLevel"))
  (return (Utilities|String|Append "Travel error: " (Utilities|String|ToString(Byte) FailureType))))