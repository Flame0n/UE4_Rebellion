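; Base unit character Blueprint with a health bar widget, a spawn fade-in and smooth turning toward attack targets.
; On BeginPlay it links the HP bar widget to itself, then a timeline drives the opacity of a dynamic material instance.
; When the timeline finishes, the mesh switches to its main material.
; SmoothFaceTo uses a timeline to lerp capsule rotation toward a given target before attacking.
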(event Custom|SmoothFaceTo
  (params (Target :type Actor%20Object%20Reference))
  ;[1 1 1] Rotate before attack
  (bind _alpha (Timeline|Rotator PlayFromStart)
    (:Update
      (Transformation|SetWorldRotation (Variables|Default|GetCapsuleComponent) (Math|Rotator|Lerp(Rotator) (Transformation|GetActorRotation) (Math|Rotator|FindLookatRotation (Transformation|GetActorLocation) (Transformation|GetActorLocation Target)) _alpha true) false false))))

(event EventBeginPlay
  ;[1 0.9234 0.609] Set up debug health widget
  (bind _ashealth_widget (Utilities|Casting|CastToHealthWidget (UserInterface|GetUserWidgetObject (Variables|Default|GetHP%20Bar))))
  (Class|UnitCharacter|SetHealthWidget _ashealth_widget)
  (Variables|/Game/Interface/Gameplay/HealthWidget.HealthWidget_C|SetOwnerPawn _ashealth_widget self)
  (bind _returnvalue (Rendering|Material|CreateDynamicMaterialInstance "/Game/Materials/MainMaterialOpaque.MainMaterialOpaque" "None" :!class /Script/Engine.KismetMaterialLibrary))
  (bind _output_get (Variables|Default|SetOpaqueMaterial _returnvalue))
  (Rendering|Material|SetMaterial (Variables|Character|GetMesh) 0 _output_get)
  (bind _opacity (Timeline|MaterialTimeline Play)
    (:Update
      (Rendering|Material|SetScalarParameterValue (Variables|Default|GetOpaqueMaterial) "Opacity" _opacity :!class /Script/Engine.MaterialInstanceDynamic))
    (:Finished
      (Rendering|Material|SetMaterial (Variables|Character|GetMesh) 0 "/Game/Materials/MainMaterial.MainMaterial"))))

(fn ConstructionScript)